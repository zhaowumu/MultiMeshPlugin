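; BP_MultiActor is an actor that builds a procedural mesh from the static meshes of two spline mesh components, apparently as a test.
; Its construction script passes both meshes as sections to MultiMeshFromStaticMeshes, with a Union operation set on the first, and writes into ProceduralMesh.
; It then prints each resulting material's name and the material count for debugging.
; The event graph holds only disabled placeholder events.
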(fn `UserConstructionScript`
  (bind _proceduralmesh (`self.ProceduralMesh`))
  (bind _returnvalue (`MeshComponent.GetMaterials` _proceduralmesh))
  (`MultiMeshLibrary.MultiMeshFromStaticMeshes` _proceduralmesh (`|MakeArray` (make `MultiMeshStaticSection` (`StaticMeshComponent.StaticMesh` (`self.SplineMesh`))) (make `MultiMeshStaticSection` (`StaticMeshComponent.StaticMesh` (`self.SplineMesh1`)) (`KismetMathLibrary.MakeTransform` (0.0 0.0 0.0)))))
  (for _array_element _returnvalue
    (`KismetSystemLibrary.PrintString` (`KismetSystemLibrary.GetDisplayName` _array_element)))
  (`KismetSystemLibrary.PrintString` (`KismetStringLibrary.Conv_IntToString` (`KismetArrayLibrary.Array_Length` _returnvalue))))